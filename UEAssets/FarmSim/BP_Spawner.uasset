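; Farm sim spawner actor that creates a fixed set of DirtPile_Blueprint rows on BeginPlay, plus a UI widget holding a reference back to it.
; UpdateDistanceBetweenRows centers the piles along the spawner's local Y axis at the given spacing.
; UpdateDistanceBetweenPlants passes plant spacing and YBounds to each pile.
; Piles are pre-spawned and toggled visible against XBounds, using local offset for row updates but world Y for plant updates.
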(event EventBeginPlay
  (for _index (range 0 32)
    (bind _returnvalue (Game|SpawnActorfromClass "/Game/Carla/Maps/FarmSim/DirtPile_Blueprint.DirtPile_Blueprint_C" (Transformation|GetActorTransform) "Undefined" 0 0))
    (Utilities|Array|Add (Variables|Default|GetInstances) _returnvalue))
  (CallFunction|UpdateDistanceBetweenRows (Variables|Default|GetDistanceBetweenRows))
  (CallFunction|UpdateDistanceBetweenPlants (Variables|Default|GetDistanceBetweenPlants))
  (bind _returnvalue_2 (UserInterface|CreateWidget "/Game/Carla/Maps/FarmSim/UI.UI_C"))
  (Variables|/Game/Carla/Maps/FarmSim/UI.UI_C|SetSpawner _returnvalue_2 self)
  (UserInterface|Viewport|AddtoViewport _returnvalue_2 0))

(event Collision|EventActorBeginOverlap
  (params (OtherActor :type Actor%20Object%20Reference)))

(event EventTick
  (params (DeltaSeconds :type Float%20%28single-precision%29)))

(fn ConstructionScript)

(fn UpdateDistanceBetweenRows
  (params (Distance :type Float%20%28single-precision%29))
  (bind _instances (Variables|Default|GetInstances))
  (bind _output_get (Variables|Default|SetDistanceBetweenRows Distance))
  (for (_array_element _array_index) _instances
    (Transformation|SetActorLocation _array_element (Math|Transform|TransformLocation (Transformation|GetActorTransform) (Math|Vector|MakeVector 0.0 (* (- _array_index (/ (Utilities|Array|Length _instances) 2)) _output_get) 0.0)) false true)
    (Default|SetDistance _array_element (Variables|Default|GetDistanceBetweenPlants))
    (Default|SetVisibilityFUNC _array_element (> (Variables|Default|GetXBounds) (Math|Float|Absolute(Float) (* (- _array_index (/ (Utilities|Array|Length _instances) 2)) _output_get))))))

(fn UpdateDistanceBetweenPlants
  (params (Distance :type Float%20%28single-precision%29))
  (bind _output_get (Variables|Default|SetDistanceBetweenPlants Distance))
  (for _array_element (Variables|Default|GetInstances)
    (Variables|/Game/Carla/Maps/FarmSim/DirtPile_Blueprint.DirtPile_Blueprint_C|SetYBounds _array_element (Variables|Default|GetYBounds))
    (Default|SetDistance _array_element _output_get)
    (Default|SetVisibilityFUNC _array_element (> (Variables|Default|GetXBounds) (Math|Float|Absolute(Float) (.Y (Math|Vector|BreakVector (Transformation|GetActorLocation _array_element))))))))